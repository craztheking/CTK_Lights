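; Fuse box Blueprint for the CTK light system that cuts its linked lights when it takes any damage.
; Damage calls ServerBroken, which passes to ClientBroken to print a debug string and loop over the Lights array.
; Each light has FuseOn cleared, and any light that is on gets toggled through its SwitchLightServer call.
; No logic here restores the fuse.
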(event Custom|Client%20Broken
  (Development|PrintString "broken")
  (for _array_element (Variables|Default|GetLights)
    (Variables|/NightOps/CTK_LightSystem/BP/BP__CTK_Light.BP__CTK_Light_C|SetFuseOn _array_element false)
    (if (Variables|/NightOps/CTK_LightSystem/BP/BP__CTK_Light.BP__CTK_Light_C|GetIsOn _array_element)
      (Default|SwitchLightServer _array_element))))

(event Custom|Server%20Broken
  (CallFunction|ClientBroken))

(event EventBeginPlay
  (|CallParentFunction))

(event Collision|EventActorBeginOverlap
  (params (OtherActor :type Actor%20Object%20Reference))
  (|CallParentFunction OtherActor) ; This node is disabled and will not be called.\nDrag off pins to build functionality.
)

(event EventTick
  (params (DeltaSeconds :type Float%20%28single-precision%29))
  (|CallParentFunction DeltaSeconds) ; This node is disabled and will not be called.\nDrag off pins to build functionality.
)

(event Game|Damage|EventAnyDamage
  (params (Damage :type Float%20%28single-precision%29) (DamageType :type Damage%20Type%20Object%20Reference) (InstigatedBy :type Controller%20Object%20Reference) (DamageCauser :type Actor%20Object%20Reference))
  (CallFunction|ServerBroken))

(fn ConstructionScript
  (|CallParentFunction))