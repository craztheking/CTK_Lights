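; Light actor that can be switched on and off or broken by damage, using either a point or spot light.
; Server-named events guard on broken state, then call Client events that swap visibility and materials, with particle and Wwise sound on break.
; Breaking from damage, optionally limited to a hitbox, and switching on both require FuseOn.
; The construction script sets up light type and hitbox; a Kelvin-to-RGB function is left unfinished.
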(event Custom|Break%20Light%20Server
  ;[1 1 1] Break Lights
  (if (not (Variables|Default|GetIsBroken))
    (Variables|Default|SetIsBroken true)
    (CallFunction|BreakLightClient)))

(event Custom|Break%20Light%20Client
  (bind _lightbroken (Variables|Default|GetLightBroken))
  ;[1 1 1] Break Lights
  (Rendering|SetVisibility (Variables|Default|GetPointLight) false false)
  (Rendering|SetVisibility _lightbroken true false)
  (Rendering|Material|SetMaterial _lightbroken 0 (Variables|Default|GetOFF%20Material))
  (Effects|SpawnEmitteratLocation (Variables|Default|GetBreak%20Particle) (Transformation|GetWorldLocation (Variables|Default|GetParticle%20Location)))
  (Class|AkGameObject|PostAkEvent (Variables|Default|GetAK) (Variables|Default|GetBreak%20Sound))
  (Variables|Default|SetIsBroken true))

(event Custom|Switch%20Light%20Server
  ;[1 1 1] Switch Lights
  (if (not (Variables|Default|GetIsBroken))
    (CallFunction|SwitchLightClient)))

(event Custom|Switch%20Light%20Client
  ;[1 1 1] Switch Lights
  (if (Variables|Default|GetIsOn)
    (if (Variables|Default|GetUseSpotLight)
      (Rendering|SetVisibility (Variables|Default|GetSpotLight) false false)
      (else
        (Rendering|SetVisibility (Variables|Default|GetPointLight) false false)))
    (Rendering|Material|SetMaterial (Variables|Default|GetLight) 0 (Variables|Default|GetOFF%20Material))
    (Variables|Default|SetIsOn false)
    (elif (not (Variables|Default|GetIsBroken))
      (if (Variables|Default|GetFuseOn)
        (if (Variables|Default|GetUseSpotLight)
          (Rendering|SetVisibility (Variables|Default|GetSpotLight) true false)
          (else
            (Rendering|SetVisibility (Variables|Default|GetPointLight) true false)))
        (Rendering|Material|SetMaterial (Variables|Default|GetLight) 0 (Variables|Default|GetOn%20Material))
        (Variables|Default|SetIsOn true)))))

(event Game|Damage|EventPointDamage
  (params (Damage :type Float%20%28single-precision%29) (DamageType :type Damage%20Type%20Object%20Reference) (HitLocation :type Vector :default "0, 0, 0") (HitNormal :type Vector :default "0, 0, 0") (HitComponent :type Primitive%20Component%20Object%20Reference) (BoneName :type Name :default "None") (ShotFromDirection :type Vector :default "0, 0, 0") (InstigatedBy :type Controller%20Object%20Reference) (DamageCauser :type Actor%20Object%20Reference) (HitInfo :type Hit%20Result%20Structure%20%28by%20ref%29))
  ;[1 1 1] Switch Lights
  (if (Variables|Default|GetUse%20Hitbox)
    (if (== HitComponent (Variables|Default|GetHitBox))
      (if (not (Variables|Default|GetIsBroken))
        (if (Variables|Default|GetFuseOn)
          (CallFunction|BreakLightServer)
          (Development|PrintString "BreakLight"))))))

(event Game|Damage|EventAnyDamage
  (params (Damage :type Float%20%28single-precision%29) (DamageType :type Damage%20Type%20Object%20Reference) (InstigatedBy :type Controller%20Object%20Reference) (DamageCauser :type Actor%20Object%20Reference))
  ;[1 1 1] Switch Lights
  (if (not (Variables|Default|GetUse%20Hitbox))
    (if (not (Variables|Default|GetIsBroken))
      (if (Variables|Default|GetFuseOn)
        (CallFunction|BreakLightServer)
        (Development|PrintString "BreakLight")))))

(fn ConstructionScript
  (bind _hitbox (Variables|Default|GetHitBox))
  (bind _spotlight (Variables|Default|GetSpotLight))
  (bind _pointlight (Variables|Default|GetPointLight))
  (bind _hitbox_2 (Variables|Default|GetHitBox))
  (Rendering|Material|SetMaterial (Variables|Default|GetLight) 0 (Variables|Default|GetOn%20Material))
  (Rendering|Material|SetMaterial (Variables|Default|GetLightBroken) 0 (Variables|Default|GetOFF%20Material))
  (if (Variables|Default|GetUseSpotLight)
    (Rendering|SetVisibility _pointlight false false)
    (Rendering|SetVisibility _spotlight true false)
    (else
      (Rendering|SetVisibility _pointlight true false)
      (Rendering|SetVisibility _spotlight false false)))
  (if (Variables|Default|GetUse%20Hitbox)
    (Collision|SetCollisionEnabled _hitbox_2 "QueryAndPhysics")
    (if (Variables|Default|GetViewHitbox)
      (Rendering|Material|SetMaterial _hitbox_2 0 "/NightOpsTest/CTK_LightSystem/Materials/M_HitBox.M_HitBox")
      (else
        (Rendering|Material|SetMaterial _hitbox_2 0 "/NightOpsTest/CTK_LightSystem/Materials/M_Invisible.M_Invisible")))
    (else
      (Rendering|Material|SetMaterial _hitbox 0 "/NightOpsTest/CTK_LightSystem/Materials/M_Invisible.M_Invisible")
      (Collision|SetCollisionEnabled _hitbox "NoCollision"))))

(fn KelvintoRGB
  (params (Tempature :type Float%20%28single-precision%29))
  (bind _output_get (LocalVariables|SetTemp (/ Tempature 1e+02)))
  ;[1 1 1] Red
  (if (not (<= _output_get 66.0))
    (LocalVariables|SetRed (- (LocalVariables|GetTemp) 6e+01))
    (bind _output_get_2 (LocalVariables|SetRed (* 329.698727446 (Math|Float|Power (LocalVariables|GetRed) -0.1332047592))))
    (if (< _output_get_2 0.0)
      (LocalVariables|SetRed 0.0)
      (elif (> (LocalVariables|GetRed) 255.0)
        (LocalVariables|SetRed 255.0)))))