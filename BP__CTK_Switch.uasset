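; Usable light switch actor that toggles a set of linked lights on and off.
; EventTryUse calls Switch, which waits on a half-second retriggerable delay, then flips LightOn.
; The On/Off "Client" events swap the visible switch component, print the state and call SwitchLightServer on each entry in Lights.
; The authority check's branches and the SwitchServer function are empty.
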(event Custom|SwitchOff%20Client
  (Rendering|SetVisibility (Variables|Default|GetLightswitch_OFF) true false)
  (Rendering|SetVisibility (Variables|Default|GetLightswitch_ON) false false)
  (Development|PrintString "Off")
  (for _array_element (Variables|Default|GetLights)
    (Default|SwitchLightServer _array_element)))

(event Custom|Switch%20On%20Client
  (Rendering|SetVisibility (Variables|Default|GetLightswitch_OFF) false false)
  (Rendering|SetVisibility (Variables|Default|GetLightswitch_ON) true false)
  (Development|PrintString "On")
  (for _array_element (Variables|Default|GetLights)
    (Default|SwitchLightServer _array_element)))

(event Custom|Switch
  (Utilities|FlowControl|RetriggerableDelay 0.5)
  (if (Variables|Default|GetLightOn)
    (Variables|Default|SetLightOn false)
    (CallFunction|SwitchOffClient)
    (else
      (Variables|Default|SetLightOn true)
      (CallFunction|SwitchonClient))))

(fn ConstructionScript)

(fn EventTryUse
  (params (Pawn :type INS%20Soldier%20Object%20Reference) (HitResult :type Hit%20Result%20Structure%20%28by%20ref%29))
  (Networking|SwitchHasAuthority
    (:Authority
      _)
    (:Remote
      _))
  (CallFunction|Switch)
  (return "HandledServer"))

(fn SwitchServer)